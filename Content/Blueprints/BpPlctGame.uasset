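; Player controller for a two-paddle Pong game that drives both paddles, runs scoring and restarts the ball.
; On BeginPlay it finds the ball and both paddles, shows the score widget and starts the ball.
; LeftControl and RightControl axes move each paddle along X within set limits, scaled by a coefficient but not by delta time.
; The ball's score event increments that side's score, stops movement, then resets and relaunches the ball after a short delay.
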(event `InputAxis|RightControl`
  (params (AxisValue :type "Float (single-precision)"))
  (bind _brightpong (`self.BRightPong`))
  (bind _returnvalue (+ (.x (`self.K2_GetActorLocation` _brightpong)) (* AxisValue (`self.BCoed`))))
  (`/Engine/EditorBlueprintResources/StandardMacros.IsValid` _brightpong
    (:`Is Valid`
      (if (and (< _returnvalue (`self.BMaxX`)) (> _returnvalue (`self.BMinX`)))
        (`self.K2_SetActorLocation` _brightpong (`KismetMathLibrary.MakeVector` _returnvalue (.y (`self.K2_GetActorLocation` _brightpong)) (.z (`self.K2_GetActorLocation` _brightpong))) false false)))))

(event `InputAxis|LeftControl`
  (params (AxisValue :type "Float (single-precision)"))
  (bind _bleftpong (`self.BLeftPong`))
  (bind _returnvalue (+ (.x (`self.K2_GetActorLocation` _bleftpong)) (* AxisValue (`self.BCoed`))))
  (`/Engine/EditorBlueprintResources/StandardMacros.IsValid` _bleftpong
    (:`Is Valid`
      (if (and (< _returnvalue (`self.BMaxX`)) (> _returnvalue (`self.BMinX`)))
        (`self.K2_SetActorLocation` _bleftpong (`KismetMathLibrary.MakeVector` _returnvalue (.y (`self.K2_GetActorLocation` _bleftpong)) (.z (`self.K2_GetActorLocation` _bleftpong))) false false)))))

(event `self.ReceiveBeginPlay`
  (`WidgetBlueprintLibrary.SetInputMode_GameOnly` self)
  (bind _outactors (`GameplayStatics.GetAllActorsOfClass` "/Game/Blueprints/BpPawnBall.BpPawnBall_C"))
  (set `self.BBallRef` (`|GetArrayItem` _outactors))
  (bind _outactors_2 (`GameplayStatics.GetAllActorsOfClass` "/Game/Blueprints/BpPawnPong.BpPawnPong_C"))
  (for _array_element _outactors_2
    (if (`/Game/Blueprints/BpPawnPong.LeftB` _array_element)
      (set `self.BLeftPong` _array_element)
      (else
        (set `self.BRightPong` _array_element))))
  (bind _returnvalue (`|CreateWidget` "/Game/Blueprints/wScore.wScore_C" self))
  (`UserWidget.AddToViewport` _returnvalue 0)
  (`self.BindBall`)
  (`/Game/Blueprints/BpPawnBall.Start` (`self.BBallRef`)))

(event `BindBall`
  (add `/Game/Blueprints/BpPawnBall.Score` (`self.BBallRef`) (delegate `Scored`)))

(event `Scored`
  (params (Left :type Boolean))
  (bind _bballref (`self.BBallRef`))
  (if Left
    (`/Engine/EditorBlueprintResources/StandardMacros.IncrementInt` (`self.BLeftScore`)
      (:`  `
        _))
    (else
      (`/Engine/EditorBlueprintResources/StandardMacros.IncrementInt` (`self.BRightScore`)
        (:`  `
          _))))
  (`KismetSystemLibrary.K2_ClearAndInvalidateTimerHandle` (`/Game/Blueprints/BpPawnBall.BTimerMove` _bballref))
  (`MovementComponent.StopMovementImmediately` (`Pawn.GetMovementComponent` _bballref))
  (`KismetSystemLibrary.Delay` 0.1)
  (`self.K2_SetActorLocation` _bballref (`self.BBallLocation`) false false)
  (`/Game/Blueprints/BpPawnBall.Start` _bballref))

(fn `UserConstructionScript`)